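; Pendulum obstacle Blueprint, apparently an old version, that lines up a row of hanging instanced meshes between BeginBox and EndBox.
; InitObstacle rebuilds the evenly spaced, flipped instances in both the construction script and BeginPlay.
; Box overlaps query IsPlayerWalkInMessage on the other actor but only clear a FirstRun flag.
; The swing logic, using MoveComponentTo and a timeline, is disconnected, so nothing moves.
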(event OnComponentBeginOverlap(beginBox)
  (params (OverlappedComponent :type Primitive%20Component%20Object%20Reference) (OtherActor :type Actor%20Object%20Reference) (OtherComp :type Primitive%20Component%20Object%20Reference) (OtherBodyIndex :type Integer) (bFromSweep :type Boolean) (SweepResult :type Hit%20Result%20Structure%20%28by%20ref%29))
  (if (Variables|Default|GetfirstRun)
    (bind _yes_no (Class|BPIPlayer|IsPlayerWalkin(Message) OtherActor))
    (if _yes_no
      (Variables|Default|SetfirstRun false))))

(event OnComponentEndOverlap(endBox)
  (params (OverlappedComponent :type Primitive%20Component%20Object%20Reference) (OtherActor :type Actor%20Object%20Reference) (OtherComp :type Primitive%20Component%20Object%20Reference) (OtherBodyIndex :type Integer)))

(event OnComponentBeginOverlap(endBox)
  (params (OverlappedComponent :type Primitive%20Component%20Object%20Reference) (OtherActor :type Actor%20Object%20Reference) (OtherComp :type Primitive%20Component%20Object%20Reference) (OtherBodyIndex :type Integer) (bFromSweep :type Boolean) (SweepResult :type Hit%20Result%20Structure%20%28by%20ref%29))
  (Variables|Default|SetfirstRun false)
  (bind _yes_no (Class|BPIPlayer|IsPlayerWalkin(Message) OtherActor))
  (if _yes_no
    _))

(event OnComponentEndOverlap(beginBox)
  (params (OverlappedComponent :type Primitive%20Component%20Object%20Reference) (OtherActor :type Actor%20Object%20Reference) (OtherComp :type Primitive%20Component%20Object%20Reference) (OtherBodyIndex :type Integer)))

(event EventBeginPlay
  (CallFunction|InitObstacle))

(event Collision|EventActorBeginOverlap
  (params (OtherActor :type Actor%20Object%20Reference)))

(event EventTick
  (params (DeltaSeconds :type Float%20%28single-precision%29)))

(fn ConstructionScript
  (CallFunction|InitObstacle))

(fn InitObstacle
  (Components|InstancedStaticMesh|ClearInstances (Variables|Default|GetmovingObjects))
  (bind _output_get (Variables|Default|SettempDistance (- (.x (Variables|/Script/Engine.SceneComponent|GetRelativeLocation (Variables|Default|GetbeginBox))) 3e+02)))
  (while (> _output_get (+ (.x (Variables|/Script/Engine.SceneComponent|GetRelativeLocation (Variables|Default|GetendBox))) 3e+02))
    (Components|InstancedStaticMesh|AddInstance (Variables|Default|GetmovingObjects) (Math|Transform|MakeTransform (Math|Vector|MakeVector _output_get 0.0 475.0) "0, 0,180.000000" "0.200000,0.200000,0.750000"))
    (Variables|Default|SettempDistance (+ (Variables|Default|GettempDistance) -2e+02))))