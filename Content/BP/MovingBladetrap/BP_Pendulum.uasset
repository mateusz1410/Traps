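; Pendulum blade trap that spawns and attaches a row of BP_Obstacle blades between BeginBox and EndBox on BeginPlay.
; The player's first BeginBox overlap starts five blades at staggered delays.
; MakeBladeMove swings each blade's roll through chained MoveComponentTo calls, repeating while Loop is true.
; EndBox's one-shot overlap clears Loop for the player, ending swings after the current cycle, and tilts each obstacle's root slightly after a delay.
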(event OnComponentBeginOverlap(beginBox)
  (params (OverlappedComponent :type Primitive%20Component%20Object%20Reference) (OtherActor :type Actor%20Object%20Reference) (OtherComp :type Primitive%20Component%20Object%20Reference) (OtherBodyIndex :type Integer) (bFromSweep :type Boolean) (SweepResult :type Hit%20Result%20Structure%20%28by%20ref%29))
  (if (Variables|Default|GetfirstRun)
    (bind _yes_no (Class|BPIPlayer|IsPlayerWalkin(Message) OtherActor))
    (if _yes_no
      (Variables|Default|SetfirstRun false)
      (Utilities|FlowControl|Sequence
        (:then_0
          (Utilities|MakeBladeMove (Utilities|Array|Get(acopy) (Variables|Default|GetmovingObject))))
        (:then_1
          (Utilities|FlowControl|Delay 1.2)
          (Utilities|MakeBladeMove (Utilities|Array|Get(acopy) (Variables|Default|GetmovingObject) 1)))
        (:then_2
          (Utilities|FlowControl|Delay 0.1)
          (Utilities|MakeBladeMove (Utilities|Array|Get(acopy) (Variables|Default|GetmovingObject) 2)))
        (:then_3
          (Utilities|FlowControl|Delay 1.3)
          (Utilities|MakeBladeMove (Utilities|Array|Get(acopy) (Variables|Default|GetmovingObject) 3)))
        (:then_4
          (Utilities|FlowControl|Delay 0.4)
          (Utilities|MakeBladeMove (Utilities|Array|Get(acopy) (Variables|Default|GetmovingObject) 4)))))))

(event OnComponentEndOverlap(endBox)
  (params (OverlappedComponent :type Primitive%20Component%20Object%20Reference) (OtherActor :type Actor%20Object%20Reference) (OtherComp :type Primitive%20Component%20Object%20Reference) (OtherBodyIndex :type Integer)))

(event OnComponentBeginOverlap(endBox)
  (params (OverlappedComponent :type Primitive%20Component%20Object%20Reference) (OtherActor :type Actor%20Object%20Reference) (OtherComp :type Primitive%20Component%20Object%20Reference) (OtherBodyIndex :type Integer) (bFromSweep :type Boolean) (SweepResult :type Hit%20Result%20Structure%20%28by%20ref%29))
  (Utilities|FlowControl|DoOnce false
    (:Completed
      (Variables|Default|SetfirstRun false)
      (bind _yes_no (Class|BPIPlayer|IsPlayerWalkin(Message) OtherActor))
      (if _yes_no
        (Variables|Default|Setloop false)
        (Utilities|FlowControl|Delay 3.0)
        (for _array_element (Variables|Default|GetmovingObject)
          (Transformation|SetRelativeTransform (Variables|/Game/BP/MovingBladetrap/BP_Obstacle.BP_Obstacle_C|GetDefaultSceneRoot _array_element) (Math|Transform|MakeTransform (.location (Transformation|GetRelativeTransform (Variables|/Game/BP/MovingBladetrap/BP_Obstacle.BP_Obstacle_C|GetDefaultSceneRoot _array_element))) (Math|Rotator|MakeRotator (Math|Float|Lerp (.roll (.rotation (Transformation|GetRelativeTransform (Variables|/Game/BP/MovingBladetrap/BP_Obstacle.BP_Obstacle_C|GetDefaultSceneRoot _array_element)))) (+ (.roll (.rotation (Transformation|GetRelativeTransform (Variables|/Game/BP/MovingBladetrap/BP_Obstacle.BP_Obstacle_C|GetDefaultSceneRoot _array_element)))) -6e+01) 0.1) (.pitch (.rotation (Transformation|GetRelativeTransform (Variables|/Game/BP/MovingBladetrap/BP_Obstacle.BP_Obstacle_C|GetDefaultSceneRoot _array_element)))) (.yaw (.rotation (Transformation|GetRelativeTransform (Variables|/Game/BP/MovingBladetrap/BP_Obstacle.BP_Obstacle_C|GetDefaultSceneRoot _array_element))))) (.scale (Transformation|GetRelativeTransform (Variables|/Game/BP/MovingBladetrap/BP_Obstacle.BP_Obstacle_C|GetDefaultSceneRoot _array_element)))) false false))))))

(event OnComponentEndOverlap(beginBox)
  (params (OverlappedComponent :type Primitive%20Component%20Object%20Reference) (OtherActor :type Actor%20Object%20Reference) (OtherComp :type Primitive%20Component%20Object%20Reference) (OtherBodyIndex :type Integer)))

(event EventBeginPlay
  (CallFunction|InitObstacle))

(event Collision|EventActorBeginOverlap
  (params (OtherActor :type Actor%20Object%20Reference)))

(event EventTick
  (params (DeltaSeconds :type Float%20%28single-precision%29)))

(fn ConstructionScript)

(fn InitObstacle
  (bind _beginbox (Variables|Default|GetbeginBox))
  (bind _endbox (Variables|Default|GetendBox))
  (bind _relativelocation (Variables|/Script/Engine.SceneComponent|GetRelativeLocation _beginbox))
  (bind _relativelocation_2 (Variables|/Script/Engine.SceneComponent|GetRelativeLocation _endbox))
  (bind (_x _y _z) (Math|Vector|BreakVector _relativelocation))
  (bind (_x_2 _y_2 _z_2) (Math|Vector|BreakVector _relativelocation_2))
  (bind _output_get (Variables|Default|SetstartRelativelocation (Math|Vector|MakeVector (+ _x -2e+02) _y _z)))
  (while (> (.X (Math|Vector|BreakVector _output_get)) (.X (Math|Vector|BreakVector (Math|Vector|MakeVector (+ _x_2 4e+02) _y_2 _z_2))))
    (bind _returnvalue (Game|SpawnActorfromClass "/Game/BP/MovingBladetrap/BP_Obstacle.BP_Obstacle_C" (Math|Transform|MakeTransform (Math|Vector|MakeVector 0.0 0.0 0.0) "0, 0, 0" "1,1,1") "Undefined" 0 0))
    (Utilities|Array|Add (Variables|Default|GetmovingObject) _returnvalue)
    (Transformation|AttachComponentToComponent _returnvalue (Variables|Default|GetbeginBox) "None" "SnapToTarget" "SnapToTarget" "KeepWorld" true)
    (Transformation|SetActorRelativeLocation _returnvalue (Math|Vector|MakeVector (* (.X (Math|Vector|BreakVector _output_get)) -1.0) (.Y (Math|Vector|BreakVector _relativelocation)) 275.0))
    (Variables|Default|SetstartRelativelocation (Math|Vector|MakeVector (- (.x (Variables|Default|GetstartRelativelocation)) 1.5e+02) (.y (Variables|Default|GetstartRelativelocation)) (.z (Variables|Default|GetstartRelativelocation))))
    (Transformation|SetActorRelativeRotation _returnvalue (Math|Rotator|MakeRotator 2e+01 0.0 0.0))))