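; Beam trap actor that drops a log and damages the player it hits.
; On BeginPlay, MoveComponentTo shifts the beam sideways and up with added roll from its relative transform.
; ActivateTrap briefly waits, then turns on physics simulation to release the beam.
; While the trap is active, a player overlapping HitBox receives hit and damage interface messages once, after which the trap is marked inactive.
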(event OnComponentBeginOverlap(HitBox)
  (params (OverlappedComponent :type Primitive%20Component%20Object%20Reference) (OtherActor :type Actor%20Object%20Reference) (OtherComp :type Primitive%20Component%20Object%20Reference) (OtherBodyIndex :type Integer) (bFromSweep :type Boolean) (SweepResult :type Hit%20Result%20Structure%20%28by%20ref%29))
  (bind _yes_no (Class|BPIPlayer|IsPlayerWalkin(Message) OtherActor))
  (if _yes_no
    (if (Variables|Default|GetIs%20Active)
      (Utilities|FlowControl|DoOnce false
        (:Completed
          (Class|BPIPlayer|Hitby(Message) OtherActor)
          (Class|BPIPlayer|AddDamage(Message) OtherActor -0.75)
          (Variables|Default|SetIs%20Active false))))))

(event EventBeginPlay
  (bind _beamsm (Variables|Default|GetbeamSM))
  (bind _returnvalue (Transformation|GetRelativeTransform _beamsm))
  (Components|MoveComponentTo _beamsm (Math|Vector|MakeVector (.x (.location _returnvalue)) (+ (.y (.location _returnvalue)) -8e+02) (+ (.z (.location _returnvalue)) 6e+02)) (Math|Rotator|MakeRotator (+ (.roll (.rotation _returnvalue)) 3e+01) (.pitch (.rotation _returnvalue)) (.yaw (.rotation _returnvalue))) false false 0.2 false))

(event Collision|EventActorBeginOverlap
  (params (OtherActor :type Actor%20Object%20Reference)))

(event EventTick
  (params (DeltaSeconds :type Float%20%28single-precision%29)))

(event EventActivateTrap
  (Utilities|FlowControl|Delay 0.2)
  (Physics|SetSimulatePhysics (Variables|Default|GetbeamSM) true))

(fn ConstructionScript)