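; BP_BeamReleaseRope is a tripwire-style rope trap trigger that can be deactivated.
; When a player passes the walk-in check on the trigger box while active, the cable end detaches and a one-shot message activates the linked ReleaseObject, disarming the rope and enabling cable collision.
; A second box passes the active trap to the player through CheckTrapMessage, clearing it on exit.
; DeactivateTrap sets the active state, detaches the cable and enables its collision.
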(event OnComponentBeginOverlap(triggerBox)
  (params (OverlappedComponent :type Primitive%20Component%20Object%20Reference) (OtherActor :type Actor%20Object%20Reference) (OtherComp :type Primitive%20Component%20Object%20Reference) (OtherBodyIndex :type Integer) (bFromSweep :type Boolean) (SweepResult :type Hit%20Result%20Structure%20%28by%20ref%29))
  (bind _releaseobject (Variables|Default|GetreleaseObject))
  (bind _yes_no (Class|BPIPlayer|IsPlayerWalkin(Message) OtherActor))
  (if _yes_no
    (if (Variables|Default|GetisActive)
      (Variables|/Script/CableComponent.CableComponent|SetbAttachEnd (Variables|Default|GetropeCable) false)
      (Utilities|FlowControl|DoOnce false
        (:Completed
          (Utilities|IsValid _releaseobject
            (:Is%20Valid
              (Class|BPITrap|ActivateTrap(Message) _releaseobject)
              (Variables|Default|SetisActive false)
              (Variables|/Script/CableComponent.CableComponent|SetbEnableCollision (Variables|Default|GetropeCable) true))))))))

(event OnComponentBeginOverlap(dectivateBox)
  (params (OverlappedComponent :type Primitive%20Component%20Object%20Reference) (OtherActor :type Actor%20Object%20Reference) (OtherComp :type Primitive%20Component%20Object%20Reference) (OtherBodyIndex :type Integer) (bFromSweep :type Boolean) (SweepResult :type Hit%20Result%20Structure%20%28by%20ref%29))
  (bind _yes_no (Class|BPIPlayer|IsPlayerWalkin(Message) OtherActor))
  (if _yes_no
    (if (Variables|Default|GetisActive)
      (Class|BPIPlayer|CheckTrap(Message) OtherActor self))))

(event OnComponentEndOverlap(dectivateBox)
  (params (OverlappedComponent :type Primitive%20Component%20Object%20Reference) (OtherActor :type Actor%20Object%20Reference) (OtherComp :type Primitive%20Component%20Object%20Reference) (OtherBodyIndex :type Integer))
  (bind _yes_no (Class|BPIPlayer|IsPlayerWalkin(Message) OtherActor))
  (if _yes_no
    (Class|BPIPlayer|CheckTrap(Message) OtherActor)))

(event EventBeginPlay)

(event Collision|EventActorBeginOverlap
  (params (OtherActor :type Actor%20Object%20Reference)))

(event EventTick
  (params (DeltaSeconds :type Float%20%28single-precision%29)))

(event EventDeactivateTrap
  (params (deactivate :type Boolean))
  (Variables|Default|SetisActive (not deactivate))
  (Variables|/Script/CableComponent.CableComponent|SetbAttachEnd (Variables|Default|GetropeCable) false)
  (Variables|/Script/CableComponent.CableComponent|SetbEnableCollision (Variables|Default|GetropeCable) true))

(fn ConstructionScript)