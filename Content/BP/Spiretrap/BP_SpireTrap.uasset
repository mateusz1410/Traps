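; Spire trap that springs once when the player enters its trigger box while it is active.
; After a short delay it quickly moves the spire mesh to its raised position and damages the player through a message call.
; A second box passes the trap to the player via CheckTrap, and DeactivateTrap toggles its active state.
; The box's end-overlap clears that reference, but runs its player check on the overlapped component instead of the other actor.
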(event OnComponentBeginOverlap(triggerBox)
  (params (OverlappedComponent :type Primitive%20Component%20Object%20Reference) (OtherActor :type Actor%20Object%20Reference) (OtherComp :type Primitive%20Component%20Object%20Reference) (OtherBodyIndex :type Integer) (bFromSweep :type Boolean) (SweepResult :type Hit%20Result%20Structure%20%28by%20ref%29))
  (bind _spiresm (Variables|Default|GetspireSM))
  (bind _returnvalue (Transformation|GetRelativeTransform _spiresm))
  (bind _yes_no (Class|BPIPlayer|IsPlayerWalkin(Message) OtherActor))
  (if _yes_no
    (if (Variables|Default|GetisActive)
      (Utilities|FlowControl|DoOnce false
        (:Completed
          (Utilities|FlowControl|Delay 0.3)
          (Components|MoveComponentTo _spiresm (Math|Vector|MakeVector (.x (.location _returnvalue)) (.y (.location _returnvalue)) 35.0) (.rotation _returnvalue) false false 0.1 false)
          (Class|BPIPlayer|AddDamage(Message) OtherActor -0.55))))))

(event OnComponentBeginOverlap(deactivateBox)
  (params (OverlappedComponent :type Primitive%20Component%20Object%20Reference) (OtherActor :type Actor%20Object%20Reference) (OtherComp :type Primitive%20Component%20Object%20Reference) (OtherBodyIndex :type Integer) (bFromSweep :type Boolean) (SweepResult :type Hit%20Result%20Structure%20%28by%20ref%29))
  (bind _yes_no (Class|BPIPlayer|IsPlayerWalkin(Message) OtherActor))
  (if _yes_no
    (if (Variables|Default|GetisActive)
      (Class|BPIPlayer|CheckTrap(Message) OtherActor self))))

(event OnComponentEndOverlap(deactivateBox)
  (params (OverlappedComponent :type Primitive%20Component%20Object%20Reference) (OtherActor :type Actor%20Object%20Reference) (OtherComp :type Primitive%20Component%20Object%20Reference) (OtherBodyIndex :type Integer))
  (bind _yes_no (Class|BPIPlayer|IsPlayerWalkin(Message) OverlappedComponent))
  (if _yes_no
    (Class|BPIPlayer|CheckTrap(Message) OtherActor)))

(event EventBeginPlay)

(event Collision|EventActorBeginOverlap
  (params (OtherActor :type Actor%20Object%20Reference)))

(event EventTick
  (params (DeltaSeconds :type Float%20%28single-precision%29)))

(event EventDeactivateTrap
  (params (deactivate :type Boolean))
  (Variables|Default|SetisActive (not deactivate)))

(fn ConstructionScript)