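; Flame trap actor that burns the player while they stand in its trigger box.
; When active, player entry turns on six fire effects and starts a Delay loop applying periodic damage by message; any actor leaving stops both.
; A second box passes the active trap to the player via CheckTrapMessage and clears it on exit.
; DeactivateTrap toggles the active flag, which is checked only on entry.
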(event OnComponentBeginOverlap(triggerBox)
  (params (OverlappedComponent :type Primitive%20Component%20Object%20Reference) (OtherActor :type Actor%20Object%20Reference) (OtherComp :type Primitive%20Component%20Object%20Reference) (OtherBodyIndex :type Integer) (bFromSweep :type Boolean) (SweepResult :type Hit%20Result%20Structure%20%28by%20ref%29))
  (bind _yes_no (Class|BPIPlayer|IsPlayerWalkin(Message) OtherActor))
  (if _yes_no
    (Variables|Default|Setplayer OtherActor)
    (if (Variables|Default|GetisActive)
      (Variables|Default|SetloopingDamage true)
      (Components|Activation|SetActive (Variables|Default|GetP_Fire1) true false)
      (if (Variables|Default|GetloopingDamage) :!label _label
        (Class|BPIPlayer|AddDamage(Message) (Variables|Default|Getplayer) -0.05)
        (Utilities|FlowControl|Delay 0.5)
        (goto _label)))))

(event OnComponentEndOverlap(triggerBox)
  (params (OverlappedComponent :type Primitive%20Component%20Object%20Reference) (OtherActor :type Actor%20Object%20Reference) (OtherComp :type Primitive%20Component%20Object%20Reference) (OtherBodyIndex :type Integer))
  (Components|Activation|SetActive (Variables|Default|GetP_Fire1) false false)
  (Variables|Default|Setplayer 0)
  (Variables|Default|SetloopingDamage false))

(event OnComponentBeginOverlap(deactivateBox)
  (params (OverlappedComponent :type Primitive%20Component%20Object%20Reference) (OtherActor :type Actor%20Object%20Reference) (OtherComp :type Primitive%20Component%20Object%20Reference) (OtherBodyIndex :type Integer) (bFromSweep :type Boolean) (SweepResult :type Hit%20Result%20Structure%20%28by%20ref%29))
  (bind _yes_no (Class|BPIPlayer|IsPlayerWalkin(Message) OtherActor))
  (if _yes_no
    (if (Variables|Default|GetisActive)
      (Class|BPIPlayer|CheckTrap(Message) OtherActor self))))

(event OnComponentEndOverlap(deactivateBox)
  (params (OverlappedComponent :type Primitive%20Component%20Object%20Reference) (OtherActor :type Actor%20Object%20Reference) (OtherComp :type Primitive%20Component%20Object%20Reference) (OtherBodyIndex :type Integer))
  (bind _yes_no (Class|BPIPlayer|IsPlayerWalkin(Message) OtherActor))
  (if _yes_no
    (Class|BPIPlayer|CheckTrap(Message) OtherActor)))

(event EventBeginPlay)

(event Collision|EventActorBeginOverlap
  (params (OtherActor :type Actor%20Object%20Reference)))

(event EventTick
  (params (DeltaSeconds :type Float%20%28single-precision%29)))

(event EventDeactivateTrap
  (params (deactivate :type Boolean))
  (Variables|Default|SetisActive (not deactivate)))

(fn ConstructionScript)