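; Single-use swinging spike arm trap that hurts the player and can be disarmed.
; While active, TriggerBox fires a fast yaw swing of the arm, then after a delay disables mesh collision and eases the arm further round.
; HitBox sends hit and damage messages once, then deactivates the trap.
; DeactivateBox passes the trap to the player via interface message and clears it on exit, with DeactivateTrap setting the active state.
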(event OnComponentBeginOverlap(triggerBox)
  (params (OverlappedComponent :type Primitive%20Component%20Object%20Reference) (OtherActor :type Actor%20Object%20Reference) (OtherComp :type Primitive%20Component%20Object%20Reference) (OtherBodyIndex :type Integer) (bFromSweep :type Boolean) (SweepResult :type Hit%20Result%20Structure%20%28by%20ref%29))
  (bind _armsm (Variables|Default|GetarmSM))
  (bind _relativerotation (Variables|/Script/Engine.SceneComponent|GetRelativeRotation _armsm))
  (bind _relativelocation (Variables|/Script/Engine.SceneComponent|GetRelativeLocation _armsm))
  (bind _yes_no (Class|BPIPlayer|IsPlayerWalkin(Message) OtherActor))
  (if _yes_no
    (if (Variables|Default|GetisActive)
      (Utilities|FlowControl|DoOnce false
        (:Completed
          (Components|MoveComponentTo _armsm _relativelocation (Math|Rotator|MakeRotator (.roll _relativerotation) (.pitch _relativerotation) (+ (.yaw _relativerotation) -115.0)) false false 0.1 false)
          (Utilities|FlowControl|Delay 3.0)
          (Collision|SetCollisionEnabled (Variables|Default|GetarmSM) "NoCollision")
          (Components|MoveComponentTo _armsm _relativelocation (Math|Rotator|MakeRotator (.roll _relativerotation) (.pitch _relativerotation) (+ (.yaw _relativerotation) -7e+01)) true false 1.5 false))))))

(event OnComponentBeginOverlap(hitBox)
  (params (OverlappedComponent :type Primitive%20Component%20Object%20Reference) (OtherActor :type Actor%20Object%20Reference) (OtherComp :type Primitive%20Component%20Object%20Reference) (OtherBodyIndex :type Integer) (bFromSweep :type Boolean) (SweepResult :type Hit%20Result%20Structure%20%28by%20ref%29))
  (bind _yes_no (Class|BPIPlayer|IsPlayerWalkin(Message) OtherActor))
  (if _yes_no
    (if (Variables|Default|GetisActive)
      (Utilities|FlowControl|DoOnce false
        (:Completed
          (Class|BPIPlayer|Hitby(Message) OtherActor)
          (Class|BPIPlayer|AddDamage(Message) OtherActor -0.6)
          (Variables|Default|SetisActive false))))))

(event OnComponentBeginOverlap(deactivateBox)
  (params (OverlappedComponent :type Primitive%20Component%20Object%20Reference) (OtherActor :type Actor%20Object%20Reference) (OtherComp :type Primitive%20Component%20Object%20Reference) (OtherBodyIndex :type Integer) (bFromSweep :type Boolean) (SweepResult :type Hit%20Result%20Structure%20%28by%20ref%29))
  (bind _yes_no (Class|BPIPlayer|IsPlayerWalkin(Message) OtherActor))
  (if _yes_no
    (if (Variables|Default|GetisActive)
      (Class|BPIPlayer|CheckTrap(Message) OtherActor self))))

(event OnComponentEndOverlap(deactivateBox)
  (params (OverlappedComponent :type Primitive%20Component%20Object%20Reference) (OtherActor :type Actor%20Object%20Reference) (OtherComp :type Primitive%20Component%20Object%20Reference) (OtherBodyIndex :type Integer))
  (bind _yes_no (Class|BPIPlayer|IsPlayerWalkin(Message) OtherActor))
  (if _yes_no
    (Class|BPIPlayer|CheckTrap(Message) OtherActor)))

(event EventBeginPlay)

(event Collision|EventActorBeginOverlap
  (params (OtherActor :type Actor%20Object%20Reference)))

(event EventTick
  (params (DeltaSeconds :type Float%20%28single-precision%29)))

(event EventDeactivateTrap
  (params (deactivate :type Boolean))
  (Variables|Default|SetisActive (not deactivate)))

(fn ConstructionScript)