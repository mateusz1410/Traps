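; Gas trap actor that hurts a player who walks into its sphere once ActivateTrap has armed it and switched on two particle systems.
; Sphere overlap identifies the player through message calls, then repeats small damage messages in a Delay-based loop.
; A parallel timer ends damage and gas after a few seconds.
; Leaving the sphere stops damage and disarms the trap immediately, then switches off particles after a delay.
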(event OnComponentEndOverlap(Sphere)
  (params (OverlappedComponent :type Primitive%20Component%20Object%20Reference) (OtherActor :type Actor%20Object%20Reference) (OtherComp :type Primitive%20Component%20Object%20Reference) (OtherBodyIndex :type Integer))
  (bind _yes_no (Class|BPIPlayer|IsPlayerWalkin(Message) OtherActor))
  (if _yes_no
    (Variables|Default|SetloopingDamage false)
    (Variables|Default|SetisActive false)
    (Utilities|FlowControl|Delay 3.0)
    (Components|Activation|SetActive (Variables|Default|GetParticleSystem) false false)
    (Variables|Default|Setplayer 0)))

(event OnComponentBeginOverlap(Sphere)
  (params (OverlappedComponent :type Primitive%20Component%20Object%20Reference) (OtherActor :type Actor%20Object%20Reference) (OtherComp :type Primitive%20Component%20Object%20Reference) (OtherBodyIndex :type Integer) (bFromSweep :type Boolean) (SweepResult :type Hit%20Result%20Structure%20%28by%20ref%29))
  (bind _yes_no (Class|BPIPlayer|IsPlayerWalkin(Message) OtherActor))
  (if _yes_no
    (Variables|Default|Setplayer OtherActor)
    (if (Variables|Default|GetisActive)
      (Variables|Default|SetloopingDamage true)
      (Utilities|FlowControl|Sequence
        (:then_0
          (if (Variables|Default|GetloopingDamage) :!label _label
            (Class|BPIPlayer|AddDamage(Message) (Variables|Default|Getplayer) -0.1)
            (Utilities|FlowControl|Delay 0.5)
            (goto _label)))
        (:then_1
          (Utilities|FlowControl|Delay 3.0)
          (Variables|Default|SetloopingDamage false)
          (Components|Activation|SetActive (Variables|Default|GetParticleSystem) false false))))))

(event EventBeginPlay)

(event Collision|EventActorBeginOverlap
  (params (OtherActor :type Actor%20Object%20Reference)))

(event EventTick
  (params (DeltaSeconds :type Float%20%28single-precision%29)))

(event EventActivateTrap
  (Variables|Default|SetisActive true)
  (Components|Activation|SetActive (Variables|Default|GetParticleSystem) true false))

(fn ConstructionScript)