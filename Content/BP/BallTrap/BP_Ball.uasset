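; Rolling ball trap actor that damages a walking player who gets caught by it.
; An active trigger overlap rotates the blocking mesh, enables its physics, then releases the physics ball with an impulse.
; A one-shot Sphere hit disables the player's capsule collision, applies damage and deactivates the trap, as does Tick once the rolling ball slows.
; DeactivateBox reports the trap to the player through interface messages, and DeactivateTrap toggles its active state.
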(event OnComponentBeginOverlap(triggerBox)
  (params (OverlappedComponent :type Primitive%20Component%20Object%20Reference) (OtherActor :type Actor%20Object%20Reference) (OtherComp :type Primitive%20Component%20Object%20Reference) (OtherBodyIndex :type Integer) (bFromSweep :type Boolean) (SweepResult :type Hit%20Result%20Structure%20%28by%20ref%29))
  (bind _blockingsm (Variables|Default|GetblockingSM))
  (bind _ball (Variables|Default|GetBall))
  (bind _returnvalue (Transformation|GetRelativeTransform _blockingsm))
  (bind _yes_no (Class|BPIPlayer|IsPlayerWalkin(Message) OtherActor))
  (if _yes_no
    (if (Variables|Default|GetisActive)
      (Utilities|FlowControl|DoOnce false
        (:Completed
          (Components|MoveComponentTo _blockingsm (.location _returnvalue) (Math|Rotator|MakeRotator (+ (.roll (.rotation _returnvalue)) 9e+01) (+ (.pitch (.rotation _returnvalue)) 1.8e+02) (.yaw (.rotation _returnvalue))) false false 0.2 false)
          (Physics|SetSimulatePhysics _blockingsm true)
          (Utilities|FlowControl|Delay 0.3)
          (Physics|SetSimulatePhysics _ball true)
          (Physics|AddImpulse _ball "0.000000,400.000000, 0" "None" true)
          (Utilities|FlowControl|Delay 0.5)
          (Variables|Default|SetisRolling true))))))

(event OnComponentEndOverlap(triggerBox)
  (params (OverlappedComponent :type Primitive%20Component%20Object%20Reference) (OtherActor :type Actor%20Object%20Reference) (OtherComp :type Primitive%20Component%20Object%20Reference) (OtherBodyIndex :type Integer)))

(event OnComponentBeginOverlap(deactivateBox)
  (params (OverlappedComponent :type Primitive%20Component%20Object%20Reference) (OtherActor :type Actor%20Object%20Reference) (OtherComp :type Primitive%20Component%20Object%20Reference) (OtherBodyIndex :type Integer) (bFromSweep :type Boolean) (SweepResult :type Hit%20Result%20Structure%20%28by%20ref%29))
  (bind _yes_no (Class|BPIPlayer|IsPlayerWalkin(Message) OtherActor))
  (if _yes_no
    (if (Variables|Default|GetisActive)
      (Class|BPIPlayer|CheckTrap(Message) OtherActor self))))

(event OnComponentEndOverlap(deactivateBox)
  (params (OverlappedComponent :type Primitive%20Component%20Object%20Reference) (OtherActor :type Actor%20Object%20Reference) (OtherComp :type Primitive%20Component%20Object%20Reference) (OtherBodyIndex :type Integer))
  (bind _yes_no (Class|BPIPlayer|IsPlayerWalkin(Message) OtherActor))
  (if _yes_no
    (Class|BPIPlayer|CheckTrap(Message) OtherActor)))

(event OnComponentBeginOverlap(Sphere)
  (params (OverlappedComponent :type Primitive%20Component%20Object%20Reference) (OtherActor :type Actor%20Object%20Reference) (OtherComp :type Primitive%20Component%20Object%20Reference) (OtherBodyIndex :type Integer) (bFromSweep :type Boolean) (SweepResult :type Hit%20Result%20Structure%20%28by%20ref%29))
  (bind _yes_no (Class|BPIPlayer|IsPlayerWalkin(Message) OtherActor))
  (if _yes_no
    (if (Variables|Default|GetisActive)
      (Utilities|FlowControl|DoOnce false
        (:Completed
          (Class|BPIPlayer|DisableCapsuleCollision(Message) OtherActor)
          (Class|BPIPlayer|AddDamage(Message) OtherActor -1.0)
          (Variables|Default|SetisActive false))))))

(event EventBeginPlay)

(event Collision|EventActorBeginOverlap
  (params (OtherActor :type Actor%20Object%20Reference)))

(event EventDeactivateTrap
  (params (deactivate :type Boolean))
  (Variables|Default|SetisActive (not deactivate)))

(event EventTick
  (params (DeltaSeconds :type Float%20%28single-precision%29))
  (if (Math|Boolean|ANDBoolean (Variables|Default|GetisActive) (<= (Math|Vector|VectorLength (Transformation|GetComponentVelocity (Variables|Default|GetBall))) 65.0) (Variables|Default|GetisRolling))
    (Variables|Default|SetisActive false)
    (Physics|SetSimulatePhysics (Variables|Default|GetBall) false)))

(fn ConstructionScript)